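; Fence gate that the player slides open and closed with the Interact input once the gate key is obtained.
; Box overlap opens and closes a Gate node, so input only passes while something overlaps the box.
; It reads GotGateKey by casting its parent actor to gate_key_bp, then a FlipFlop plays or reverses a timeline that drives the mesh's relative X location.
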(event `InputAction|Interact`
  (params (Key :type "Key Structure"))
  (:`Pressed`
    (`/Engine/EditorBlueprintResources/StandardMacros.Gate` true :!label _label
      (:`Exit`
        (bind _asgate_key_bp (cast `/Game/Forest_Stuff/gate_key_bp` (`self.GetParentActor`)))
        (if (`/Game/Forest_Stuff/gate_key_bp.Got_Gate_Key` _asgate_key_bp)
          (`/Engine/EditorBlueprintResources/StandardMacros.FlipFlop`
            (:`A`
              (bind (_direction _fence_open_) (`Timeline|gate_open` :!label _label_2)
                (:`Update`
                  (`SceneComponent.K2_SetRelativeLocation` (`self.StaticMesh`) (`KismetMathLibrary.MakeVector` _fence_open_) false false))))
            (:`B`
              (goto _label_2 :!via `Reverse`))))))))

(event `self.Box.OnComponentBeginOverlap`
  (params (OverlappedComponent :type "PrimitiveComponent Object Reference") (OtherActor :type "Actor Object Reference") (OtherComp :type "PrimitiveComponent Object Reference") (OtherBodyIndex :type Integer) (bFromSweep :type Boolean) (SweepResult :type "HitResult Structure (by ref)"))
  (goto _label :!via `Open`))

(event `self.Box.OnComponentEndOverlap`
  (params (OverlappedComponent :type "PrimitiveComponent Object Reference") (OtherActor :type "Actor Object Reference") (OtherComp :type "PrimitiveComponent Object Reference") (OtherBodyIndex :type Integer))
  (goto _label :!via `Close`))

(event `self.ReceiveBeginPlay`
  (`self.EnableInput` (`GameplayStatics.GetPlayerController` 0)))

(fn `UserConstructionScript`)